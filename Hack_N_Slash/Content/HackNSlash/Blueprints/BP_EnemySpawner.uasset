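; BP_EnemySpawner is a trigger actor that spawns a group of enemies when the player first overlaps it.
; It reads a class-to-count map, places each enemy at a random navigable point within Radius, and yaws it toward the player, drawing a debug sphere of the area.
; It tallies spawned enemies, and IncreaseDeaths shows the WB_Victory widget once deaths reach that total.
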(event EventBeginPlay)

(event Collision|EventActorBeginOverlap
  (params (OtherActor :type Actor%20Object%20Reference))
  (Utilities|FlowControl|DoOnce false
    (:Completed
      (bind _asbp_player (Utilities|Casting|CastToBP_Player OtherActor))
      (Variables|Default|Setplayer _asbp_player)
      (CallFunction|Spawn))))

(event EventTick
  (params (DeltaSeconds :type Float%20%28single-precision%29)))

(fn ConstructionScript)

(fn Spawn
  (bind _keys (Utilities|Map|Keys (Variables|Default|GetEnemiesToSpawn)))
  (for _array_element _keys
    (for _index (range 1 (.Value (Utilities|Map|Find (Variables|Default|GetEnemiesToSpawn) _array_element)))
      (bind _randomlocation (Class|NavigationSystemV1|GetRandomLocationinNavigableRadius (Transformation|GetActorLocation) (Variables|Default|Getradius) 0 0))
      (bind _returnvalue (Game|SpawnActorfromClass _array_element (Math|Transform|MakeTransform _randomlocation "0, 0, 0" "1.000000,1.000000,1.000000") "AdjustIfPossibleButAlwaysSpawn" "MultiplyWithRoot" 0 0))
      (Transformation|SetActorRotation _returnvalue (Math|Rotator|MakeRotator (.roll (Transformation|GetActorRotation _returnvalue)) (.pitch (Transformation|GetActorRotation _returnvalue)) (.yaw (Math|Rotator|FindLookatRotation (Transformation|GetActorLocation _returnvalue) (Transformation|GetActorLocation (Variables|Default|Getplayer))))))
      (Rendering|Debug|DrawDebugSphere (Transformation|GetActorLocation) (Variables|Default|Getradius) 18 "(R=1.000000,G=0.000000,B=0.000000,A=1.000000)" 1e+01 5.0)
      (Variables|Default|SettotalEnemies (+ (Variables|Default|GettotalEnemies) 1)))))

(fn IncreaseDeaths
  (bind _output_get (Variables|Default|Setdeaths (+ (Variables|Default|Getdeaths) 1)))
  (if (>= _output_get (Variables|Default|GettotalEnemies))
    (bind _returnvalue (UserInterface|CreateWidget "/Game/HackNSlash/Blueprints/UI/WB_Victory.WB_Victory_C" (Game|GetPlayerController 0)))
    (UserInterface|Viewport|AddtoViewport _returnvalue 0)))