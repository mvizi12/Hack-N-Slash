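; Base AI controller for HackNSlash enemies that reacts when its AI Perception detects the player by sight or damage.
; Perception updates for BP_Player actors run two checks in sequence, calling HandleSensedSight or HandleSensedDamage when the matching one passes.
; CanSensePlayer maps a sense enum to its AISense class and passes only if the stimulus matches that class and was successfully sensed, so lost-sense updates trigger neither handler.
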(event OnTargetPerceptionUpdated(AIPerception)
  (params (Actor :type Actor%20Object%20Reference) (Stimulus :type AI%20Stimulus%20Structure))
  (bind _asbp_player (Utilities|Casting|CastToBP_Player Actor))
  (Utilities|IsValid _asbp_player
    (:Is%20Valid
      (Variables|Default|Setplayer _asbp_player)
      (Utilities|FlowControl|Sequence
        (:then_0
          (bind _sensed_ (CallFunction|CanSensePlayer (Variables|Default|Getplayer) Stimulus "SightSense"))
          (if _sensed_
            (Class|EnemyBaseController|HandleSensedSight (Variables|Default|Getplayer))))
        (:then_1
          (bind _sensed__2 (CallFunction|CanSensePlayer (Variables|Default|Getplayer) Stimulus "DamageSense"))
          (if _sensed__2
            (Class|EnemyBaseController|HandleSensedDamage (Variables|Default|Getplayer))))))))

(fn ConstructionScript)

(fn CanSensePlayer
  (params (player :type Actor%20Object%20Reference) (stimulus :type AI%20Stimulus%20Structure) (sense :type EAISense%20Enum :default "NoneSense"))
  (bind _returnvalue (Class|AIPerceptionSystem|GetSenseClassforStimulus stimulus))
  (if (== _returnvalue (Utilities|Select :Index sense :NoneSense 0 :SightSense "/Script/AIModule.AISense_Sight" :DamageSense "/Script/AIModule.AISense_Damage"))
    (return (.bSuccessfullySensed (Utilities|Struct|BreakAIStimulus stimulus)))
    (else
      (return false))))