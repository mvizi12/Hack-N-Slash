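; Base enemy Blueprint with a socket-attached sword, health handling, lock-on display and launch reactions.
; Incoming damage with a DamageTypeMain type goes to the Stats component, whose delegates update the health bar widget and trigger death handling.
; Selection events toggle the lock-on and health bar widgets.
; CombatEnemy's launch delegate drives a timeline feeding alpha into LaunchEnemy; landing stops it, disables collision and tries an attack reset.
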(event OnHealthPercentUpdateDelegate(Stats)
  (params (newPercent :type Float%20%28single-precision%29))
  (bind _healthbar (Variables|Default|GethealthBar))
  (Utilities|IsValid _healthbar
    (:Is%20Valid
      (Default|SetPercentage _healthbar newPercent))))

(event OnZeroHealthUpdateDelegate(Stats)
  (Class|EnemyBase|HandleDeath))

(event OnLaunchEnemyDelegate(CombatEnemy)
  (params (distance :type Vector :default "0, 0, 0"))
  ;[1 1 1 0.5] Launch Enemy
  (CallFunction|ResetTimelines)
  (bind _alpha (Timeline|Launch%20TL PlayFromStart)
    (:Update
      (Class|CombatEnemyComponent|LaunchEnemy (Variables|Default|GetCombatEnemy) distance _alpha))))

(event EventBeginPlay
  (CallFunction|AttatchWeapon)
  (CallFunction|GetHBWidget))

(event EventOnSelect
  (Rendering|SetVisibility (Variables|Default|GetWidgetLockOn) true true)
  (Rendering|SetVisibility (Variables|Default|GetWidgetHealthBar) true true))

(event EventOnLanded
  (params (Hit :type Hit%20Result%20Structure%20%28by%20ref%29))
  (CallFunction|ResetTimelines)
  (Class|EnemyBase|DisableCollision)
  (Class|CombatEnemyComponent|TryResetAttack (Variables|Default|GetCombatEnemy)))

(event Game|Damage|EventAnyDamage
  (params (Damage :type Float%20%28single-precision%29) (DamageType :type Damage%20Type%20Object%20Reference) (InstigatedBy :type Controller%20Object%20Reference) (DamageCauser :type Actor%20Object%20Reference))
  (CallFunction|HandleDamage Damage DamageType DamageCauser))

(event EventOnDeselect
  (Rendering|SetVisibility (Variables|Default|GetWidgetLockOn) false true)
  (Rendering|SetVisibility (Variables|Default|GetWidgetHealthBar) false true))

(fn ConstructionScript)

(fn AttatchWeapon
  (bind _returnvalue (Game|SpawnActorfromClass "/Game/HackNSlash/Blueprints/BP_Sword_Tanjiro.BP_Sword_Tanjiro_C" (Transformation|GetSocketTransform (Variables|Character|GetMesh) "weapon_hand_start_r" "RTS_World") "Undefined" "MultiplyWithRoot" self 0))
  (Transformation|AttachComponentToComponent _returnvalue (Variables|Character|GetMesh) "weapon_hand_start_r" "SnapToTarget" "SnapToTarget" "SnapToTarget" true))

(fn GetHBWidget
  (bind _aswb_enemy_hb (Utilities|Casting|CastToWB_EnemyHB (UserInterface|GetWidget (Variables|Default|GetWidgetHealthBar))))
  (bind _output_get (Variables|Default|SethealthBar _aswb_enemy_hb))
  (Utilities|IsValid _output_get
    (:Is%20Valid
      (Default|SetPercentage _output_get (Class|StatsComponent|GetStatPercentage (Variables|Default|GetStats) "Health" "MaxHealth")))))

(fn HandleDamage
  (params (damage :type Float%20%28single-precision%29) (Object :type Object%20Object%20Reference) (opponent :type Actor%20Object%20Reference))
  (bind _asdamage_type_main (Utilities|Casting|CastToDamageTypeMain Object))
  (Class|StatsComponent|ReduceHealth (Variables|Default|GetStats) damage (Class|DamageTypeMain|GetBuffer _asdamage_type_main) opponent (Class|DamageTypeMain|GetDamageType _asdamage_type_main)))

(fn ResetTimelines
  (Audio|Components|Audio|Stop (Variables|Default|GetLaunch%20TL)))